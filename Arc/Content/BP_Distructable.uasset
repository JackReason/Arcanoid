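; Destructible block that takes hits from BP_Ball and drops a bonus when destroyed, as in a brick-breaker.
; Each ball hit increments a counter and switches the cube to a golden material until the count reaches Lives, then the actor is destroyed.
; On destruction it randomly spawns BP_Bonus1 or BP_Bonus2 at the cube transform cached on BeginPlay, with the drop chance currently set to always.
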(event `self.ReceiveBeginPlay`
  (set `self.LocationBonus` (`SceneComponent.K2_GetComponentToWorld` (`self.Cube`))))

(event `self.ReceiveHit`
  (params (MyComp :type "PrimitiveComponent Object Reference") (Other :type "Actor Object Reference") (OtherComp :type "PrimitiveComponent Object Reference") (bSelfMoved :type Boolean) (HitLocation :type "Vector Structure") (HitNormal :type "Vector Structure") (NormalImpulse :type "Vector Structure") (Hit :type "HitResult Structure (by ref)"))
  (bind _locationbonus (`self.LocationBonus`))
  (cast `/Game/BP_Ball` Other)
  (bind _result (`/Engine/EditorBlueprintResources/StandardMacros.IncrementInt` (`self.Hits`))
    (:`  `
      (if (< _result (`self.Lives`))
        (`KismetSystemLibrary.PrintString` (`KismetStringLibrary.Concat_StrStr` "Hits: " (`KismetStringLibrary.Conv_IntToString` _result)))
        (`PrimitiveComponent.SetMaterial` (`self.Cube`) 0 "/Game/BP_Golden.BP_Golden")
        (else
          (`self.K2_DestroyActor`)
          (`KismetSystemLibrary.PrintString` "Distroyed!")
          (if (`KismetMathLibrary.RandomBoolWithWeight` 1.0)
            (switch `int` (`KismetMathLibrary.RandomInteger` 2)
              (:`0`
                (`|SpawnActorFromClass` "/Game/BP_Bonus1.BP_Bonus1_C" _locationbonus "AlwaysSpawn" "MultiplyWithRoot" null null))
              (:`1`
                (`|SpawnActorFromClass` "/Game/BP_Bonus2.BP_Bonus2_C" _locationbonus "AlwaysSpawn" "MultiplyWithRoot" null null)))))))))

(fn `UserConstructionScript`)