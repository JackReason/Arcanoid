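; BP_Ball is a bouncing ball actor that moves at Speed along Direction and dies when it leaves a KillZVolume.
; Each Tick it moves its Sphere component with a swept world offset scaled by delta time, without using physics forces.
; On a blocking hit it reflects Direction about the surface normal.
; Ending overlap with a KillZVolume calls the OnDead dispatcher, then destroys the actor.
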(event `self.ReceiveActorEndOverlap`
  (params (OtherActor :type "Actor Object Reference"))
  (cast `KillZVolume` OtherActor)
  (`self.OnDead`)
  (`self.K2_DestroyActor`))

(event `self.ReceiveTick`
  (params (DeltaSeconds :type "Float (single-precision)"))
  (bind _sweephitresult (`SceneComponent.K2_AddWorldOffset` (`self.Sphere`) (* DeltaSeconds (* (`self.Direction`) (`self.Speed`))) true false))
  (bind (_bblockinghit _binitialoverlap _time _distance _location _impactpoint _normal) (`GameplayStatics.BreakHitResult` _sweephitresult))
  (if _bblockinghit
    (set `self.Direction` (`KismetMathLibrary.GetReflectionVector` (`self.Direction`) _normal))))

(fn `UserConstructionScript`)