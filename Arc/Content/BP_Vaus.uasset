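; BP_Vaus is the player paddle of a ball game with lives, spawning and tracking the ball.
; MoveRight input slides it along X by a fixed swept offset per axis event, using only the sign of the value.
; On BeginPlay it spawns a BP_Ball at its Sphere component and binds the ball's OnDead event.
; Each death decrements Lives, then either respawns a ball or prints game over at zero.
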(event `InputAxis|MoveRight`
  (params (AxisValue :type "Float (single-precision)"))
  (if (< AxisValue 0.0)
    (`self.K2_AddActorWorldOffset` (-5.0 0.0 0.0) true)))

(event `InputAxis|MoveRight`
  (params (AxisValue :type "Float (single-precision)"))
  (if (> AxisValue 0.0)
    (`self.K2_AddActorWorldOffset` (5.0 0.0 0.0) true)))

(event `self.ReceiveBeginPlay`
  (bind _returnvalue (`|SpawnActorFromClass` "/Game/BP_Ball.BP_Ball_C" (`KismetMathLibrary.MakeTransform` (`SceneComponent.K2_GetComponentLocation` (`self.Sphere`))) "AlwaysSpawn" "MultiplyWithRoot" null null :!label _label))
  (bind _output_get (set `self.Ball` _returnvalue))
  (add `/Game/BP_Ball.OnDead` _output_get (delegate `EventDead`)))

(event `EventDead`
  (bind _result (`/Engine/EditorBlueprintResources/StandardMacros.DecrementInt` (`self.Lives`))
    (:`  `
      (bind _output_get (set `self.Lives` _result))
      (if (== _output_get 0)
        (`KismetSystemLibrary.PrintString` "Game over!")
        (else
          (goto _label))))))

(fn `UserConstructionScript`)